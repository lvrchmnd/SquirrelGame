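; Game instance for the Squirrel game that holds the quest list and tracks each quest's status.
; On Init it copies DT_QuestList rows into QuestList, which functions expose for reading, starting and ending quests by ID.
; Lookups go through SearchQuestList, which as written returns after checking only the first entry.
; EndQuest reads fields using the ID as index, and its end-target dialog loop is unfinished.
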(event EventInit
  ;[0 1 0] Read quest table into QuestList
  (bind _outrownames (DataTable|GetDataTableRowNames "/Game/Data/DT_QuestList.DT_QuestList"))
  (for _array_element _outrownames
    (bind _returnvalue (Utilities|GetDataTableRow "/Game/Data/DT_QuestList.DT_QuestList" _array_element)
      (:then
        (Utilities|Array|Add (Variables|Default|GetQuestList) _returnvalue)))))

(fn SearchQuestList
  (params (InputID :type Integer))
  (for (_array_element _array_index) (Variables|Default|GetQuestList)
    (if (== (.id _array_element) InputID)
      (return InputID _array_index)
      (else
        (return InputID -1)))))

(fn EndQuest
  (params (QuestID :type Integer))
  ;[0 1 0] Set Quest to completed
  (bind (_foundid _index) (CallFunction|SearchQuestList QuestID))
  (if (!= _index -1)
    (Utilities|Array|SetArrayElem (Variables|Default|GetQuestList) _index (Utilities|Struct|MakeFQuests (.id (Utilities|Array|Get(acopy) (Variables|Default|GetQuestList) _foundid)) (.name (Utilities|Array|Get(acopy) (Variables|Default|GetQuestList) _foundid)) (.description (Utilities|Array|Get(acopy) (Variables|Default|GetQuestList) _foundid)) "NewEnumerator2" (.endtargets (Utilities|Array|Get(acopy) (Variables|Default|GetQuestList) _foundid))))
    ;[0 1 0] SetNPCDialog - loop End Targets - NOT DONE!!
    (for _array_element (.endtargets (Utilities|Array|Get(acopy) (Variables|Default|GetQuestList) _foundid))
      _)
    (return true)
    (else
      (return false))))

(fn GetQuest
  (params (QuestID :type Integer))
  ;[0 1 0] Search then return a Quest record.
  (bind _index (CallFunction|SearchQuestList QuestID))
  (if (!= _index -1)
    (return (Utilities|Array|Get(acopy) (Variables|Default|GetQuestList) _index) true)
    (else
      (return "" false))))

(fn GetQuestList
  ;[0 1 0] Return Quest List.
  (return (Variables|Default|GetQuestList)))

(fn GetQuestStatus
  (params (QuestID :type Integer))
  ;[0 1 0] Return Quest Status (Used?)
  (bind _index (CallFunction|SearchQuestList QuestID))
  (if (!= _index -1)
    (return (.status (Utilities|Array|Get(acopy) (Variables|Default|GetQuestList) _index)) true)
    (else
      (return "NewEnumerator0" false))))

(fn StartQuest
  (params (QuestID :type Integer))
  ;[0 1 0] Set Quest to Started.
  (bind _index (CallFunction|SearchQuestList QuestID))
  (if (!= _index -1)
    (Utilities|Array|SetArrayElem (Variables|Default|GetQuestList) _index (Utilities|Struct|MakeFQuests (.id (Utilities|Array|Get(acopy) (Variables|Default|GetQuestList) _index)) (.name (Utilities|Array|Get(acopy) (Variables|Default|GetQuestList) _index)) (.description (Utilities|Array|Get(acopy) (Variables|Default|GetQuestList) _index)) "NewEnumerator1" (.endtargets (Utilities|Array|Get(acopy) (Variables|Default|GetQuestList) _index))))
    (return true)
    (else
      (return false))))