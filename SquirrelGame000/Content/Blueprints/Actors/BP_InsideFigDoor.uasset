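; BP_InsideFigDoor is an interactable door that teleports the squirrel player from inside the fig to outside it.
; A sphere overlap toggles the interact widget and registers or clears the door as the player's interactable actor.
; Interact plays a fade timeline, moves the player to a hardcoded transform, then reverses a second fade timeline.
; Both timelines drive a FadeMaterial parameter, but the nodes assigning that material are disconnected.
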(event OnComponentBeginOverlap(Sphere)
  (params (OverlappedComponent :type Primitive%20Component%20Object%20Reference) (OtherActor :type Actor%20Object%20Reference) (OtherComp :type Primitive%20Component%20Object%20Reference) (OtherBodyIndex :type Integer) (bFromSweep :type Boolean) (SweepResult :type Hit%20Result%20Structure%20%28by%20ref%29))
  (bind _player (Variables|Default|GetPlayer))
  ;[1 0 0 0] Show interact widget and send interactable actor
  (if (== OtherActor _player)
    (Rendering|SetVisibility (Variables|Default|GetWidget) true false)
    (Class|BPIInteract|SetInteractableActor(Message) _player self)))

(event OnComponentEndOverlap(Sphere)
  (params (OverlappedComponent :type Primitive%20Component%20Object%20Reference) (OtherActor :type Actor%20Object%20Reference) (OtherComp :type Primitive%20Component%20Object%20Reference) (OtherBodyIndex :type Integer))
  (bind _player (Variables|Default|GetPlayer))
  ;[1 0 0 0] Hide interact widget and clear interactable actor
  (if (== OtherActor _player)
    (Rendering|SetVisibility (Variables|Default|GetWidget) false false)
    (Class|BPIInteract|SetInteractableActor(Message) _player)))

(event EventBeginPlay
  ;[1 0 0 0] Store player to prevent errant overlaps.
  (bind _asbp_squirrel (Utilities|Casting|CastToBP_Squirrel (Game|GetPlayerCharacter 0)))
  (Variables|Default|SetPlayer _asbp_squirrel)
  (Variables|Default|SetOutsideFigDoor (Math|Transform|MakeTransform "5160.000000,-4077.000000,264.000000" "0, 0, 0" "1.000000,1.000000,1.000000"))
  (Variables|Default|SetInsideFigDoor (Math|Transform|MakeTransform "13175.000000,15298.000000,-442.000000" "0, 0, 0" "1.000000,1.000000,1.000000")))

(event EventInteract
  (bind _fadevalue (Timeline|Fade2BlackTimeline Play)
    (:Update
      (Rendering|Material|SetScalarParameterValue (Variables|Default|GetFadeMaterial) "Fade" _fadevalue :!class /Script/Engine.MaterialInstanceDynamic))
    (:Finished
      (Transformation|SetActorTransform (Variables|Default|GetPlayer) (Variables|Default|GetOutsideFigDoor))
      (bind _fadevalue_2 (Timeline|Timeline_0 Reverse)
        (:Update
          (Rendering|Material|SetScalarParameterValue (Variables|Default|GetFadeMaterial) "Fade" _fadevalue_2 :!class /Script/Engine.MaterialInstanceDynamic))))))

(fn ConstructionScript)