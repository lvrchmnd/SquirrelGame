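; Trigger volume actor that switches BP_Squirrel into 2D mode while it overlaps the box and back out when it leaves.
; On entry it compares the box's world X and Y scale and stores the box location on the longer axis in TriggerBoxCoords; equal scales trigger nothing.
; Both entry and exit set the squirrel's Is2DMode and call its CameraSwitcher, with debug prints along the way.
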(event OnComponentBeginOverlap(2DTriggerBox)
  (params (OverlappedComponent :type Primitive%20Component%20Object%20Reference) (OtherActor :type Actor%20Object%20Reference) (OtherComp :type Primitive%20Component%20Object%20Reference) (OtherBodyIndex :type Integer) (bFromSweep :type Boolean) (SweepResult :type Hit%20Result%20Structure%20%28by%20ref%29))
  (bind _returnvalue (Transformation|GetWorldScale OverlappedComponent))
  (bind _output_get (Variables|Default|SetX2DTriggerValue (.x _returnvalue)))
  (bind _output_get_2 (Variables|Default|SetY2DTriggerValue (.y _returnvalue)))
  (Development|PrintString "Overlap")
  (Math|Float|CompareFloat _output_get _output_get_2
    (:>
      (Variables|Default|SetTriggerBoxCoords (.x (Transformation|GetWorldLocation OverlappedComponent)))
      (bind _asbp_squirrel (Utilities|Casting|CastToBP_Squirrel OtherActor)
        (:then
          (Variables|/Game/Blueprints/Characters/BP_Squirrel.BP_Squirrel_C|SetIs2DMode _asbp_squirrel true)
          (Default|CameraSwitcher _asbp_squirrel))
        (:CastFailed
          (Development|PrintString "castFailed" :!label _label))))
    (:<
      (Variables|Default|SetTriggerBoxCoords (.y (Transformation|GetWorldLocation OverlappedComponent)))
      (bind _asbp_squirrel_2 (Utilities|Casting|CastToBP_Squirrel OtherActor)
        (:then
          (Variables|/Game/Blueprints/Characters/BP_Squirrel.BP_Squirrel_C|SetIs2DMode _asbp_squirrel_2 true)
          (Default|CameraSwitcher _asbp_squirrel_2))
        (:CastFailed
          (goto _label))))))

(event OnComponentEndOverlap(2DTriggerBox)
  (params (OverlappedComponent :type Primitive%20Component%20Object%20Reference) (OtherActor :type Actor%20Object%20Reference) (OtherComp :type Primitive%20Component%20Object%20Reference) (OtherBodyIndex :type Integer))
  (bind _asbp_squirrel (Utilities|Casting|CastToBP_Squirrel OtherActor))
  (Variables|/Game/Blueprints/Characters/BP_Squirrel.BP_Squirrel_C|SetIs2DMode _asbp_squirrel false)
  (Development|PrintString "EndOverlap")
  (Default|CameraSwitcher _asbp_squirrel))

(event EventBeginPlay)

(event Collision|EventActorBeginOverlap
  (params (OtherActor :type Actor%20Object%20Reference)))

(event EventTick
  (params (DeltaSeconds :type Float%20%28single-precision%29)))

(fn ConstructionScript)