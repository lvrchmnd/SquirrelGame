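; BP_Switch is an interactable switch that relays the squirrel player's interaction to a target actor.
; It caches the player as BP_Squirrel on BeginPlay so that only that character triggers the sphere overlap.
; Overlap shows or hides a prompt widget and sets or clears the switch as the player's interactable actor.
; Its Interact event forwards an interact message to InteractTarget if valid, with no animation implemented despite the graph comment.
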(event OnComponentBeginOverlap(Sphere)
  (params (OverlappedComponent :type Primitive%20Component%20Object%20Reference) (OtherActor :type Actor%20Object%20Reference) (OtherComp :type Primitive%20Component%20Object%20Reference) (OtherBodyIndex :type Integer) (bFromSweep :type Boolean) (SweepResult :type Hit%20Result%20Structure%20%28by%20ref%29))
  (bind _player (Variables|Default|GetPlayer))
  ;[1 0 0 0] Show interact widget and send interactable actor
  (if (== OtherActor _player)
    (Rendering|SetVisibility (Variables|Default|GetWidget) true false)
    (Class|BPIInteract|SetInteractableActor(Message) _player self)))

(event OnComponentEndOverlap(Sphere)
  (params (OverlappedComponent :type Primitive%20Component%20Object%20Reference) (OtherActor :type Actor%20Object%20Reference) (OtherComp :type Primitive%20Component%20Object%20Reference) (OtherBodyIndex :type Integer))
  (bind _player (Variables|Default|GetPlayer))
  ;[1 0 0 0] Hide interact widget and clear interactable actor
  (if (== OtherActor _player)
    (Rendering|SetVisibility (Variables|Default|GetWidget) false false)
    (Class|BPIInteract|SetInteractableActor(Message) _player)))

(event EventBeginPlay
  ;[1 0 0 0] Store player to prevent errant overlaps.
  (bind _asbp_squirrel (Utilities|Casting|CastToBP_Squirrel (Game|GetPlayerCharacter 0)))
  (Variables|Default|SetPlayer _asbp_squirrel))

(event EventInteract
  ;[1 0 0 0] Do interaction - play anim - get interact target - send interact command to target.
  (bind _interacttarget (Variables|Default|GetInteractTarget)
    (:then
      (Class|BPIInteract|Interact(Message) _interacttarget))
    (:else)))

(fn ConstructionScript)