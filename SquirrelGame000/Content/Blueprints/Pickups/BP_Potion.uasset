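; BP_Potion is a pickup that passes its name, icon and amount to the BP_Squirrel player character when collected.
; Any overlap on its Sphere, with no check on the other actor, plays sound and Niagara effects, disables collision and calls CollectItemMessage on the player cached at BeginPlay.
; WinkOut runs a timeline that scales and vertically offsets the Cylinder, then destroys the actor.
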(event OnComponentBeginOverlap(Sphere)
  (params (OverlappedComponent :type Primitive%20Component%20Object%20Reference) (OtherActor :type Actor%20Object%20Reference) (OtherComp :type Primitive%20Component%20Object%20Reference) (OtherBodyIndex :type Integer) (bFromSweep :type Boolean) (SweepResult :type Hit%20Result%20Structure%20%28by%20ref%29))
  (bind _returnvalue (Transformation|GetActorLocation))
  ;[1 0 0 0] Overllap and effects
  (Audio|SpawnSoundatLocation "/Game/Assets/Sounds/Pickups/SW_Pickup1.SW_Pickup1" _returnvalue "0, 0, 0" 1.0 1.0 0.0 0 0)
  (Niagara|SpawnSystematLocation "/Game/Niagara/NS_Pickup.NS_Pickup" _returnvalue)
  (CallFunction|WinkOut)
  (Collision|SetCollisionEnabled (Variables|Default|GetSphere) "NoCollision")
  ;[0 1 0 0] Colect Item
  (Class|BPIInteract|CollectItem(Message) (Variables|Default|GetPlayer) (Variables|Default|GetName) (Variables|Default|GetIcon) (Variables|Default|GetAmount))
  (Development|PrintString "Called Collect!!"))

(event Custom|WinkOut
  (bind _returnvalue (Transformation|GetActorLocation))
  (bind _cylinder (Variables|Default|GetCylinder))
  ;[1 0 0 0] WinkOut
  (bind (_direction _scale _location) (Timeline|PickupTimeline Play)
    (:Update
      (Transformation|SetWorldScale3D _cylinder (Math|Vector|MakeVector _scale _scale _scale))
      (Transformation|SetWorldLocation _cylinder (Math|Vector|MakeVector (.x _returnvalue) (.y _returnvalue) (+ (.z _returnvalue) (* _location 1e+02))) false false))
    (:Finished
      (Actor|DestroyActor))))

(event EventBeginPlay
  ;[1 0 0 0] Store Player variable
  (bind _asbp_squirrel (Utilities|Casting|CastToBP_Squirrel (Game|GetPlayerCharacter 0)))
  (Variables|Default|SetPlayer _asbp_squirrel))

(fn ConstructionScript)