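; BP_ScanActor runs an area scan effect from the actor's location.
; StartScan sets the timeline play rate from the requested duration and, unless already scanning, captures the starting location and plays the timeline.
; Each update writes the animated radius and that fixed origin to the PC_ScanCollection material parameter collection, so materials can read the scan.
; When the timeline finishes, it clears IsScanning and fires the scanning-completed callback.
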(event Custom|StartScan
  (params (ScanDuration :type Float%20%28double-precision%29))
  (Components|Timeline|SetPlayRate (Variables|Default|GetScanTimeline) (CallFunction|CalculateTimelinePlayRatebyDuration ScanDuration))
  (if (not (Variables|Default|GetIsScanning))
    (Variables|Default|SetScanStartingLocation (Transformation|GetActorLocation))
    (bind _floattrack (Timeline|ScanTimeline PlayFromStart)
      (:Update
        (Rendering|Material|SetScalarParameterValue "/Game/Defender/Demo/Materials/MaterialParameters/PC_ScanCollection.PC_ScanCollection" "Radius" _floattrack :!class /Script/Engine.KismetMaterialLibrary)
        (Rendering|Material|SetVectorParameterValue "/Game/Defender/Demo/Materials/MaterialParameters/PC_ScanCollection.PC_ScanCollection" "PlayerLocation" (Utilities|Struct|MakeLinearColor (.x (Variables|Default|GetScanStartingLocation)) (.y (Variables|Default|GetScanStartingLocation)) (.z (Variables|Default|GetScanStartingLocation)) 1.0) :!class /Script/Engine.KismetMaterialLibrary))
      (:Finished
        (Variables|Default|SetIsScanning false)
        (Default|CallOnScanningCompleted self)))))

(fn ConstructionScript)