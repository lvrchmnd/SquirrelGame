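; BP_LevelManager feeds player, wind and water values into Material Parameter Collections for the level's materials.
; Every Tick it writes player 0's location and forward vector to MyPlayerPosition.
; It also converts WDirection from degrees to a direction vector and writes it, with WSpeed as intensity, to WindBasic.
; The construction script writes WaterLevel to MyPlayerPosition as WaterZLevel, so water height is not refreshed on Tick.
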(event EventBeginPlay)

(event Collision|EventActorBeginOverlap
  (params (OtherActor :type Actor%20Object%20Reference)))

(event EventTick
  (params (DeltaSeconds :type Float%20%28single-precision%29))
  (bind _returnvalue (Math|Trig|GetPI))
  (bind _returnvalue_2 (Game|GetPlayerCharacter 0))
  (bind _w_direction (Variables|Default|GetW_Direction))
  (bind _returnvalue_3 (* _w_direction _returnvalue))
  (bind _returnvalue_4 (/ _returnvalue_3 1.8e+02))
  (Rendering|Material|SetVectorParameterValue "/Game/StylizedEnvironment/Material/MaterialParameterCollection/MyPlayerPosition.MyPlayerPosition" "PlayerPos" (Math|Conversions|ToLinearColor(Vector) (Transformation|GetActorLocation _returnvalue_2)) :!class /Script/Engine.KismetMaterialLibrary)
  (Rendering|Material|SetVectorParameterValue "/Game/StylizedEnvironment/Material/MaterialParameterCollection/MyPlayerPosition.MyPlayerPosition" "PlayerForward" (Math|Conversions|ToLinearColor(Vector) (Transformation|GetActorForwardVector _returnvalue_2)) :!class /Script/Engine.KismetMaterialLibrary)
  (Rendering|Material|SetVectorParameterValue "/Game/StylizedEnvironment/Material/MaterialParameterCollection/WindBasic.WindBasic" "W_Direction" (Utilities|Struct|MakeLinearColor (Math|Trig|Cos(Radians) _returnvalue_4) (Math|Trig|Sin(Radians) _returnvalue_4) 1.0 0.0) :!class /Script/Engine.KismetMaterialLibrary)
  (Rendering|Material|SetScalarParameterValue "/Game/StylizedEnvironment/Material/MaterialParameterCollection/WindBasic.WindBasic" "W_Intensity" (Variables|Default|GetW_Speed) :!class /Script/Engine.KismetMaterialLibrary))

(fn ConstructionScript
  (Rendering|Material|SetScalarParameterValue "/Game/StylizedEnvironment/Material/MaterialParameterCollection/MyPlayerPosition.MyPlayerPosition" "WaterZLevel" (Variables|Default|GetWaterLevel) :!class /Script/Engine.KismetMaterialLibrary))